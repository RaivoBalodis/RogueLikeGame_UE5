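; BP_EnemySpawner is a wave-system actor that spawns queued enemy classes at its own transform.
; AddEnemy queues a class and spawns immediately if no AI_Joe overlaps its sphere, while a looping timer also attempts spawns without that check.
; Successful spawns leave the queue, bind an elimination event and are tracked for ClearEnemies to destroy.
; Enemydestroyed reports deaths to the game mode.
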(event Custom|Enemydestroyed
  (Default|OnEnemyDead (CallFunction|GetPlayerGameGamemode)))

(event Custom|AddEnemy
  (params (EnemyToAdd :type AI%20Joe%20Class%20Reference%20%28by%20ref%29))
  (Utilities|Array|Add (Variables|Default|GetEnemy) EnemyToAdd)
  (if (not (Utilities|Array|IsValidIndex (Collision|GetOverlappingActors (Variables|Default|GetSphere) "/Game/AI_System/AI_Joe.AI_Joe_C" :!class /Script/Engine.PrimitiveComponent)))
    (CallFunction|FSpawnEnemy)))

(event Custom|ClearEnemies
  (for _array_element (Variables|Default|GetSpawnedEnemy)
    (Utilities|IsValid _array_element
      (:Is%20Valid
        (Actor|DestroyActor _array_element)))))

(event Custom|TrySpawnEnemy
  (CallFunction|FSpawnEnemy))

(event EventBeginPlay
  (Utilities|Time|SetTimerbyEvent (delegate Custom|TrySpawnEnemy) 5.0 true))

(fn ConstructionScript)

(fn FSpawnEnemy
  (if (Utilities|Array|IsValidIndex (Variables|Default|GetEnemy))
    (bind _returnvalue (Game|SpawnActorfromClass (Utilities|Array|Get(acopy) (Variables|Default|GetEnemy)) (Transformation|GetActorTransform) "AdjustIfPossibleButAlwaysSpawn" "MultiplyWithRoot" 0 2e+01 2.5e+02 1e+02 0))
    (Utilities|IsValid _returnvalue
      (:Is%20Valid
        (EventDispatchers|BindEventtoEliminated _returnvalue (EventDispatchers|CreateEvent :!event Custom|Enemydestroyed))
        (Utilities|Array|RemoveIndex (Variables|Default|GetEnemy))
        (Utilities|Array|Add (Variables|Default|GetSpawnedEnemy) 0)
        (return true))
      (:Is%20Not%20Valid
        (Development|PrintString "Hello")))))