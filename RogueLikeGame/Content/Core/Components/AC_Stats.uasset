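; Actor component that tracks XP and levels, updating the player HUD's XP bar.
; XP gains trigger level-ups that raise the next threshold by a fixed amount and chain while XP remains.
; Levels divisible by a target interval queue a card selection widget, switching to UI-only input and halting movement; other levels play a level-up animation.
; An interface callback removes closed card widgets and reopens one for remaining pending levels.
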(event Custom|CheckPendingLevels
  (bind _returnvalue (Game|GetPlayerController 0))
  (Utilities|IsValid (Variables|Default|GetWB_Cards)
    (:Is%20Valid
      (CallFunction|CheckLevelUp))
    (:Is%20Not%20Valid
      (bind _returnvalue_2 (UserInterface|CreateWidget "/Game/Core/Player/Widget/WB_Cards.WB_Cards_C" (Game|GetPlayerController 0)))
      (Variables|Default|SetWB_Cards _returnvalue_2)
      (UserInterface|Viewport|AddtoViewport _returnvalue_2 0)
      (Variables|/Script/Engine.PlayerController|SetbShowMouseCursor _returnvalue true)
      (Input|SetInputModeUIOnly _returnvalue (Variables|Default|GetWB_Cards) "DoNotLock" false)
      (Class|BPICharacter|ISetMovementMode(Message) (Game|GetPlayerCharacter 0) "MOVE_None")
      (CallFunction|CheckLevelUp))))

(event Custom|CheckLevelUp
  (if (>= (Variables|Default|GetCurrentXP) (Variables|Default|GetMaxXp))
    (Stats|XP|FIncreeseLevel))
  (Default|SetPercent (Variables|Default|GetWB_PlayerWidget) (Variables|Default|GetCurrentXP) (Variables|Default|GetMaxXp)))

(event EventICheckPendingLevel
  (params (ClosedWidget? :type Boolean))
  (if ClosedWidget?
    (Widget|RemovefromParent (Variables|Default|GetWB_Cards))
    (Variables|Default|SetWB_Cards 0)
    (if (>= (Variables|Default|GetPendingLevels) 2)
      (Utilities|FlowControl|Delay 0.5)
      (Math|Integer|DecrementInt (Variables|Default|GetPendingLevels)
        (:%20%20
          (CallFunction|CheckPendingLevels)))
      (else
        (Math|Integer|DecrementInt (Variables|Default|GetPendingLevels))))))

(event EventBeginPlay
  (Utilities|FlowControl|DelayUntilNextTick)
  (if (Variables|Default|GetIsPlayer?)
    (bind _asbp_first_person_character (Utilities|Casting|CastToBP_FirstPersonCharacter (Game|GetPlayerCharacter 0)))
    (Variables|Default|SetBP_Player _asbp_first_person_character)
    (bind _output_get (Variables|Default|SetWB_PlayerWidget (Variables|/Game/FirstPerson/Blueprints/BP_FirstPersonCharacter.BP_FirstPersonCharacter_C|GetWB_PlayerHud _asbp_first_person_character)))
    (Default|SetPercent _output_get (Variables|Default|GetCurrentXP) (Variables|Default|GetMaxXp))))

(fn FIncreeseXP
  (params (XP :type Float%20%28double-precision%29))
  (Variables|Default|SetCurrentXP (+ (Variables|Default|GetCurrentXP) XP))
  (if (>= (Variables|Default|GetCurrentXP) (Variables|Default|GetMaxXp))
    (Stats|XP|FIncreeseLevel))
  (Default|SetPercent (Variables|Default|GetWB_PlayerWidget) (Variables|Default|GetCurrentXP) (Variables|Default|GetMaxXp)))

(fn FDecreeseXP)

(fn FIncreeseLevel
  (bind _currentlevel (Variables|Default|GetCurrentLevel))
  (bind _output_get (Variables|Default|SetCurrentXP (- (Variables|Default|GetCurrentXP) (Variables|Default|GetMaxXp))))
  (Math|Integer|IncrementInt (Variables|Default|GetCurrentLevel)
    (:%20%20
      (bind _output_get_2 (Variables|Default|SetMaxXp (+ (Variables|Default|GetMaxXp) 1.5e+02)))
      (Default|SetPercent (Variables|Default|GetWB_PlayerWidget) _output_get _output_get_2)
      (if (== (Math|Integer|%(Integer) _currentlevel (Variables|Default|GetTragetLevel)) 0)
        (Math|Integer|IncrementInt (Variables|Default|GetPendingLevels)
          (:%20%20
            (CallFunction|CheckPendingLevels)))
        (else
          (Default|LevelUpAnim (Variables|/Game/Core/Player/Widget/WB_MainHud.WB_MainHud_C|GetWB_LevelUp (Variables|Default|GetWB_PlayerWidget)) 3.0 _currentlevel)
          (CallFunction|CheckLevelUp))))))